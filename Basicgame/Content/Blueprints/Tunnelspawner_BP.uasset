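; Tunnel spawner actor that builds an endless-runner style chain of Tunnel_BP segments, starting with several pieces at BeginPlay.
; The first segment spawns at the player character's location, and each later one at the newest tunnel's Spawnlocation point.
; Every new segment becomes NewestTunnel, receives a reference back to the spawner, and runs its Spawnwall function.
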(event EventBeginPlay
  (CallFunction|SpawnInitialTunnels))

(event Collision|EventActorBeginOverlap
  (params (OtherActor :type Actor%20Object%20Reference)))

(event EventTick
  (params (DeltaSeconds :type Float%20%28single-precision%29)))

(fn ConstructionScript)

(fn Spawntunnel
  (params (Location :type Vector))
  (bind _returnvalue (Game|SpawnActorfromClass "/Game/Blueprints/Tunnel_BP.Tunnel_BP_C" (Math|Transform|MakeTransform Location "0, 0, 0" "1.000000,1.000000,1.000000") "Undefined" "MultiplyWithRoot" 0 0))
  (bind _output_get (Variables|Default|Setnewest%20tunnel _returnvalue))
  (Variables|/Game/Blueprints/Tunnel_BP.Tunnel_BP_C|Settunnelspawnerref _output_get self)
  (Default|Spawnwall _output_get))

(fn SpawnTunnelatSpawnPoint
  (CallFunction|Spawntunnel (Transformation|GetWorldLocation (Variables|/Game/Blueprints/Tunnel_BP.Tunnel_BP_C|Getspawnlocation (Variables|Default|Getnewest%20tunnel)))))

(fn SpawnInitialTunnels
  (for _index (range 0 3)
    (Utilities|IsValid (Variables|Default|Getnewest%20tunnel)
      (:Is%20Valid
        (CallFunction|SpawnTunnelatSpawnPoint))
      (:Is%20Not%20Valid
        (CallFunction|Spawntunnel (Transformation|GetActorLocation (Game|GetPlayerCharacter 0)))))))