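; Tunnel segment actor for an endless-tunnel game, with a rotating holed wall that ends the game when it hits Player_BP.
; Spawnwall picks one of four hole meshes at random and gives it a random starting roll; Tick keeps it spinning at Rotationspeed.
; When the player overlaps the Box trigger, the segment asks its spawner reference for a new tunnel and destroys itself.
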(event OnComponentBeginOverlap(Box)
  (params (OverlappedComponent :type Primitive%20Component%20Object%20Reference) (OtherActor :type Actor%20Object%20Reference) (OtherComp :type Primitive%20Component%20Object%20Reference) (OtherBodyIndex :type Integer) (bFromSweep :type Boolean) (SweepResult :type Hit%20Result%20Structure%20%28by%20ref%29))
  (Utilities|Casting|CastToPlayer_BP OtherActor)
  (Default|SpawnTunnelatSpawnPoint (Variables|Default|Gettunnelspawnerref))
  (Actor|DestroyActor))

(event OnComponentHit(wall)
  (params (HitComponent :type Primitive%20Component%20Object%20Reference) (OtherActor :type Actor%20Object%20Reference) (OtherComp :type Primitive%20Component%20Object%20Reference) (NormalImpulse :type Vector :default "0, 0, 0") (Hit :type Hit%20Result%20Structure%20%28by%20ref%29))
  (bind _asplayer_bp (Utilities|Casting|CastToPlayer_BP OtherActor))
  (Default|GameOver _asplayer_bp))

(event EventBeginPlay)

(event Collision|EventActorBeginOverlap
  (params (OtherActor :type Actor%20Object%20Reference)))

(event EventTick
  (params (DeltaSeconds :type Float%20%28single-precision%29))
  (Transformation|AddLocalRotation (Variables|Default|Getwall) (Math|Rotator|MakeRotator (* DeltaSeconds (Variables|Default|GetRotationspeed)) 0.0 0.0) false false))

(fn ConstructionScript)

(fn Spawnwall
  (Components|StaticMesh|SetStaticMesh (Variables|Default|Getwall) (Utilities|Select :Index (Math|Random|RandomIntegerinRange 0 3) :Option%200 "/Game/Meshes/SM_Hole_04.SM_Hole_04" :Option%201 "/Game/Meshes/SM_Hole_01.SM_Hole_01" :Option%202 "/Game/Meshes/SM_Hole_02.SM_Hole_02" :Option%203 "/Game/Meshes/SM_Hole_03.SM_Hole_03"))
  (Transformation|AddLocalRotation (Variables|Default|Getwall) (Math|Rotator|MakeRotator (Math|Random|RandomFloatinRange 0.0 3.6e+02) 0.0 0.0) false false))